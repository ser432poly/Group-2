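; Behavior tree task that picks a random wander destination for the Enemy2_Random AI.
; After a random delay of up to a few seconds, it casts the owner to AIController1 and turns off sprinting on its controlled pawn.
; It then writes a random reachable point around the owner's location to the DestLocation blackboard key and finishes successfully.
; A failed cast leaves the task unfinished.
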(event EventReceiveExecute
  (params (OwnerActor :type Actor%20Object%20Reference))
  (Utilities|FlowControl|Delay (Math|Random|RandomFloatinRange 0.0 3.0))
  (bind _asaicontroller_1 (Utilities|Casting|CastToAIController1 OwnerActor))
  (bind _asenemy_2_random (Utilities|Casting|CastToEnemy2_Random (Pawn|GetControlledPawn _asaicontroller_1)))
  (Variables|/Game/MainBlueprints/Blueprints/Enemy2_Random.Enemy2_Random_C|SetisSprinting _asenemy_2_random false)
  (AI|BehaviorTree|SetBlackboardValueasVector (Variables|Default|GetdestLocation) (AI|Navigation|GetRandomReachablePointinRadius (Transformation|GetActorLocation OwnerActor) 3e+03))
  (AI|BehaviorTree|FinishExecute true))