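; Enemy character that chases the seen pawn and shoots projectiles at it, with health scaled to the player's level.
; PawnSensing triggers movement toward the pawn and a delayed projectile spawn from the mesh's Shoot socket.
; Projectile hits on the Box subtract their Power from health; at exactly zero, Tick destroys the enemy, and Destroyed adds score to the player.
; Tick also sets walk speed from a sprint flag.
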(event OnComponentHit(Box)
  (params (OtherActor :type Actor%20Object%20Reference) (OtherComp :type Primitive%20Component%20Object%20Reference) (NormalImpulse :type Vector :default "0, 0, 0") (Hit :type Hit%20Result%20Structure%20%28by%20ref%29))
  (bind _asfirst_person_projectile (Utilities|Casting|CastToFirstPersonProjectile OtherActor))
  (Variables|Default|SetCurHealth (- (Variables|Default|GetCurHealth) (Variables|/Game/FirstPersonBP/Blueprints/FirstPersonProjectile.FirstPersonProjectile_C|GetPower _asfirst_person_projectile)))
  (Actor|DestroyActor _asfirst_person_projectile))

(event OnSeePawn(PawnSensing)
  (params (Pawn :type Pawn%20Object%20Reference))
  (AI|Navigation|SimpleMovetoActor (Pawn|GetController) Pawn)
  (CallFunction|Fire))

(event Custom|Fire
  (Utilities|FlowControl|Delay 0.2)
  (Game|SpawnActorfromClass "/Game/FirstPersonBP/Blueprints/FirstPersonProjectile.FirstPersonProjectile_C" (Transformation|GetSocketTransform (Variables|Character|GetMesh self) "Shoot" "RTS_World") "Undefined" 0 0))

(event EventTick
  (params (DeltaSeconds :type Float%20%28single-precision%29))
  (bind _charactermovement (Variables|Character|GetCharacterMovement))
  (if (Variables|Default|GetisSprinting)
    (Variables|/Script/Engine.CharacterMovementComponent|SetMaxWalkSpeed _charactermovement 6e+02)
    (else
      (Variables|/Script/Engine.CharacterMovementComponent|SetMaxWalkSpeed _charactermovement 1.5e+02)))
  (if (== (Variables|Default|GetCurHealth) 0)
    (Physics|SetSimulatePhysics (Variables|Character|GetMesh) true)
    (Actor|DestroyActor)))

(event EventBeginPlay
  (bind _asthird_person_character (Utilities|Casting|CastToThirdPersonCharacter (Game|GetPlayerCharacter 0)))
  (bind _output_get (Variables|Default|SetMaxHealth (+ (Variables|/Game/ThirdPersonCPP/Blueprints/ThirdPersonCharacter.ThirdPersonCharacter_C|Getlevel _asthird_person_character) 2)))
  (Variables|Default|SetCurHealth _output_get))

(event EventDestroyed
  (bind _asthird_person_character (Utilities|Casting|CastToThirdPersonCharacter (Game|GetPlayerCharacter 0)))
  (Variables|/Game/ThirdPersonCPP/Blueprints/ThirdPersonCharacter.ThirdPersonCharacter_C|SetScore _asthird_person_character (+ (Variables|/Game/ThirdPersonCPP/Blueprints/ThirdPersonCharacter.ThirdPersonCharacter_C|GetScore _asthird_person_character) 100)))

(fn ConstructionScript
  (|CallParentFunction))