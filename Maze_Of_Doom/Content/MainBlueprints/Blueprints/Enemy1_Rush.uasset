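; Rushing enemy that chases the player with simple move-to while alive and fires projectiles from its Shoot socket after a short delay when it sees a pawn.
; Its health and projectile power scale with the player's Level.
; Player projectiles hitting its Box subtract the player's Power.
; At zero health it ragdolls and is destroyed after a delay, adding to the player's Score on destruction.
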(event OnComponentHit(Box)
  (params (OtherActor :type Actor%20Object%20Reference) (OtherComp :type Primitive%20Component%20Object%20Reference) (NormalImpulse :type Vector :default "0, 0, 0") (Hit :type Hit%20Result%20Structure%20%28by%20ref%29))
  (bind _asfirst_person_projectile (Utilities|Casting|CastToFirstPersonProjectile OtherActor))
  (bind _asthird_person_character (Utilities|Casting|CastToThirdPersonCharacter (Game|GetPlayerCharacter 0)))
  (Variables|Default|SetCurHealth (- (Variables|Default|GetCurHealth) (Variables|/Game/ThirdPersonCPP/Blueprints/ThirdPersonCharacter.ThirdPersonCharacter_C|GetPower _asthird_person_character)))
  (Actor|DestroyActor _asfirst_person_projectile))

(event OnSeePawn(PawnSensing)
  (params (Pawn :type Pawn%20Object%20Reference))
  (AI|Navigation|SimpleMovetoActor (Pawn|GetController) Pawn)
  (CallFunction|Fire))

(event Custom|Fire
  (Utilities|FlowControl|Delay 0.25)
  (bind _returnvalue (Game|SpawnActorfromClass "/Game/FirstPersonBP/Blueprints/EnemyProjectile.EnemyProjectile_C" (Transformation|GetSocketTransform (Variables|Character|GetMesh self) "Shoot" "RTS_World") "Undefined" 0 0))
  (bind _asthird_person_character (Utilities|Casting|CastToThirdPersonCharacter (Game|GetPlayerCharacter 0)))
  (Variables|/Game/FirstPersonBP/Blueprints/EnemyProjectile.EnemyProjectile_C|SetPower _returnvalue (Variables|/Game/ThirdPersonCPP/Blueprints/ThirdPersonCharacter.ThirdPersonCharacter_C|Getlevel _asthird_person_character)))

(event EventTick
  (params (DeltaSeconds :type Float%20%28single-precision%29))
  (if (<= (Variables|Default|GetCurHealth) 0)
    (Input|DisableInput 0)
    (Physics|SetSimulatePhysics (Variables|Character|GetMesh) true)
    (Utilities|FlowControl|Delay 2.0)
    (Actor|DestroyActor)
    (else
      (AI|Navigation|SimpleMovetoActor (Pawn|GetController) (Game|GetPlayerCharacter 0)))))

(event EventDestroyed
  (bind _asthird_person_character (Utilities|Casting|CastToThirdPersonCharacter (Game|GetPlayerCharacter 0)))
  (Variables|/Game/ThirdPersonCPP/Blueprints/ThirdPersonCharacter.ThirdPersonCharacter_C|SetScore _asthird_person_character (+ (Variables|/Game/ThirdPersonCPP/Blueprints/ThirdPersonCharacter.ThirdPersonCharacter_C|GetScore _asthird_person_character) 100)))

(event EventBeginPlay
  (bind _asthird_person_character (Utilities|Casting|CastToThirdPersonCharacter (Game|GetPlayerCharacter 0)))
  (bind _output_get (Variables|Default|SetMaxHealth (Variables|/Game/ThirdPersonCPP/Blueprints/ThirdPersonCharacter.ThirdPersonCharacter_C|Getlevel _asthird_person_character)))
  (Variables|Default|SetCurHealth _output_get))

(fn ConstructionScript
  (|CallParentFunction))